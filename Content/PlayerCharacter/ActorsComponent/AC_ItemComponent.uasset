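; Player character component that handles focusing, interacting with and using items.
; Each tick it line-traces using the character's camera data, storing and notifying any hit actor that implements BPI_Interact.
; Interacting makes that actor the current item and sends it an interact message through InteractingOnServ.
; RepNotify action flags trigger the current item's first action and pass the second-action state to the character's animation instance.
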(event `self.ReceiveBeginPlay`
  (bind _playercharacter (message `/Game/PlayerCharacter/BPI_PlayerCharacterLink.getPlayerCharacter` (`self.GetOwner`)))
  (set `self.Player Character` _playercharacter))

(event `self.ReceiveTick`
  (params (DeltaSeconds :type "Float (single-precision)"))
  (`self.InteractionTrace`))

(event `Interacting`
  (bind _hit_actor (`self.Hit Actor`)
    (:`then`
      (bind _output_get (set `self.currentItem` _hit_actor))
      (`self.InteractingOnServ` _output_get (`self.Player Character`)))
    (:`else`)))

(event `InteractingOnServ`
  (params (Target :type "/Game/Items/BP_Item Object Reference") (interactor :type "/Game/PlayerCharacter/BP_PlayerCharacter Object Reference"))
  (message `/Game/PlayerCharacter/Interfaces/BPI_Interact.interact` Target interactor))

(fn `InteractionTrace`
  (bind _playercharacter (message `/Game/PlayerCharacter/BPI_PlayerCharacterLink.getPlayerCharacter` (`self.GetOwner`)))
  (bind (_start _end) (`/Game/PlayerCharacter/BP_PlayerCharacter.getCamRadius` _playercharacter))
  (bind (_outhit _returnvalue) (`KismetSystemLibrary.LineTraceSingle` :`Start` _start :`End` _end :`TraceChannel` "TraceTypeQuery3" :`DrawDebugType` "ForOneFrame"))
  (if _returnvalue
    (bind (_bblockinghit _binitialoverlap _time _distance _location _impactpoint _normal _impactnormal _physmat _hitactor) (`GameplayStatics.BreakHitResult` _outhit))
    (if (`KismetSystemLibrary.DoesImplementInterface` _hitactor "/Game/PlayerCharacter/Interfaces/BPI_Interact.BPI_Interact_C")
      (bind _item (message `/Game/Items/BPI_ItemsLink.getItem` _hitactor))
      (set `self.Hit Actor` _item)
      (message `/Game/PlayerCharacter/Interfaces/BPI_Interact.onFocused` _hitactor)
      (else
        (set `self.Hit Actor` null)))))

(fn `OnRep_isFirstAction`
  (if (`self.isFirstAction`)
    (bind _currentitem (`self.currentItem`)
      (:`then`
        (`/Game/Items/BP_Item.firstAction` _currentitem))
      (:`else`))))

(fn `OnRep_isSecondAction`
  (message `/Game/PlayerCharacter/Interfaces/BPI_Anims.I_SecondAction` (`SkeletalMeshComponent.GetAnimInstance` (`Character.Mesh` (`self.Player Character`))) (`self.isSecondAction`)))