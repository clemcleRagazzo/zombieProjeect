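; Actor component that manages the player's stamina and switches the character's walk speed between sprint and walk.
; Sprint drains stamina on each call while moving, and UpdateStamina clamps the value and broadcasts it, with IsAdding true for zero or negative amounts.
; A self-calling delayed regen loop starts at BeginPlay and ends once it finds the player sprinting.
; The restart call after UnSprint is unconnected, so regen does not resume.
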(event `self.ReceiveBeginPlay`
  (bind _playercharacter (message `/Game/PlayerCharacter/BPI_PlayerCharacterLink.getPlayerCharacter` (`self.GetOwner`)))
  (set `self.Player Character` _playercharacter)
  (`self.incrementStamina`))

(event `incrementStamina`
  (if (not (`/Game/PlayerCharacter/BP_PlayerCharacter.isSprinting` (`self.Player Character`)))
    (`self.updateStamina` 0.5)
    (`KismetSystemLibrary.Delay` 1.0)
    (`self.incrementStamina`)))

(fn `sprint`
  (bind _player_character (`self.Player Character`))
  (set `CharacterMovementComponent.MaxWalkSpeed` (`/Game/PlayerCharacter/BP_PlayerCharacter.sprintSpeed` _player_character) (`Character.CharacterMovement` _player_character))
  (if (`/Game/PlayerCharacter/BP_PlayerCharacter.isMoving` _player_character)
    (`self.updateStamina` -0.05)))

(fn `unSprint`
  (bind _player_character (`self.Player Character`))
  (set `CharacterMovementComponent.MaxWalkSpeed` (`/Game/PlayerCharacter/BP_PlayerCharacter.walkSpeed` _player_character) (`Character.CharacterMovement` _player_character)))

(fn `updateStamina`
  (params (staminaAmount :type "Float (double-precision)"))
  (bind _maxstamina (`self.maxStamina`))
  (bind _output_get (set `self.stamina` (`KismetMathLibrary.FClamp` (+ (`self.stamina`) staminaAmount) 0.0 _maxstamina)))
  (`self.onStaminaChanged` _output_get _maxstamina (<= staminaAmount 0.0)))