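; AC_HealthComponent is an actor component that manages the player character's health, damage, healing and death.
; Damage and healing clamp CurrentHealth and fire OnHealthChanged, with both ignored once health reaches zero.
; Zero health or Kill runs Die, which fires OnDeath and ragdolls the owner cached at BeginPlay; Kill leaves health unchanged.
; A RepNotify on CurrentHealth rebroadcasts changes, while the MaxHealth notify is empty.
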(event `self.ReceiveBeginPlay`
  (bind _playercharacter (message `/Game/PlayerCharacter/BPI_PlayerCharacterLink.getPlayerCharacter` (`self.GetOwner`)))
  (set `self.Player Character` _playercharacter))

(fn `die`
  (`self.onDeath`)
  (`/Game/PlayerCharacter/BP_PlayerCharacter.ragDoll` (`self.Player Character`))
  (return))

(fn `heal`
  (params (healAmount :type "Float (double-precision)"))
  (bind _maxhealth (`self.maxHealth`))
  (if (`self.isDead`)
    (return)
    (else
      (bind _output_get (set `self.currentHealth` (`KismetMathLibrary.FClamp` (+ healAmount (`self.currentHealth`)) 0.0 _maxhealth)))
      (`self.onHealthChanged` _output_get _maxhealth)
      (if (`self.isDead`)
        (`self.die`)
        (return)))))

(fn `isDead`
  (returns (isDead :type Boolean))
  (return (<= (`self.currentHealth`) 0.0)))

(fn `kill`
  (`self.die`))

(fn `NewFunction`)

(fn `OnRep_currentHealth`
  (`self.onHealthChanged` (`self.currentHealth`) (`self.maxHealth`))
  (`KismetSystemLibrary.PrintString` "A pelle"))

(fn `OnRep_maxHealth`)

(fn `takeDammage`
  (params (dammageAmount :type "Float (double-precision)"))
  (bind _maxhealth (`self.maxHealth`))
  (if (`self.isDead`)
    (return)
    (else
      (bind _output_get (set `self.currentHealth` (`KismetMathLibrary.FClamp` (- (`self.currentHealth`) dammageAmount) 0.0 _maxhealth)))
      (if (== _output_get 0.0)
        (`self.onHealthChanged` 0.0)
        (`self.die`)
        (return)
        (else
          (`self.onHealthChanged` _output_get _maxhealth)
          (return))))))