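; Player interactor component that detects the actor at the camera and shows its item message in the WBP_InteractItem widget.
; BeginPlay caches the widget through a timed reference lookup.
; InteractionTrace box-traces on Visibility, stores the hit actor, and updates or resets the prompt.
; The trace's forward offset is multiplied by zero, and nothing in this component calls InteractionTrace.
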(event `self.ReceiveBeginPlay`
  (bind _widgetref (`/Game/PlayerCharacter/ActorsComponent/BML_Interaction.getWidgetReference` "/Game/UID/Interact/WBP_InteractItem.WBP_InteractItem_C" 10)
    (:`true`
      (bind _aswbp_interact_item (cast `/Game/UID/Interact/WBP_InteractItem` _widgetref))
      (set `self.As WBP Interact Item` _aswbp_interact_item))))

(fn `InteractionTrace`
  (bind _returnvalue (`GameplayStatics.GetPlayerCameraManager` 0))
  (bind _returnvalue_2 (`Actor.K2_GetActorLocation` _returnvalue))
  (bind (_outhit _returnvalue_3) (`KismetSystemLibrary.BoxTraceSingle` _returnvalue_2 (+ _returnvalue_2 (* (`Actor.GetActorForwardVector` _returnvalue) (0.0 0.0 0.0))) (10.0 10.0 10.0) (struct) "TraceTypeQuery1"))
  (if _returnvalue_3
    (bind _output_get (set `self.Hit Actor` (`.HitActor` (`GameplayStatics.BreakHitResult` _outhit))))
    (bind _item (message `/Game/Items/BPI_ItemsLink.getItem` _output_get))
    (`/Game/UID/Interact/WBP_InteractItem.update` (`self.As WBP Interact Item`) _item true)
    (else
      (`self.Hit Actor`
        (:`then`
          (set `self.Hit Actor` null)
          (`/Game/UID/Interact/WBP_InteractItem.update` (`self.As WBP Interact Item`) null))
        (:`else`)))))