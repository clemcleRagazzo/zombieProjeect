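; Actor component that tracks a player character's thirst, draining it over time and refilling it when drinking.
; From BeginPlay, a self-calling event with a Delay lowers Thirst by a fixed amount on a repeating interval.
; UpdateThirst and Drink subtract or add to Thirst, clamp it between zero and MaxThirst, and broadcast OnThirstChanged with the new and maximum values.
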(event `self.ReceiveBeginPlay`
  (`self.decrementThirst`))

(event `decrementThirst`
  (`self.updateThirst` 1.0)
  (`KismetSystemLibrary.Delay` 2.0)
  (`self.decrementThirst`))

(fn `drink`
  (params (drinkAmout :type "Float (double-precision)"))
  (bind _maxthirst (`self.maxThirst`))
  (bind _output_get (set `self.thirst` (`KismetMathLibrary.FClamp` (+ drinkAmout (`self.thirst`)) 0.0 _maxthirst)))
  (`self.onThirstChanged` _output_get _maxthirst))

(fn `updateThirst`
  (params (thirstAmount :type "Float (double-precision)"))
  (bind _maxthirst (`self.maxThirst`))
  (bind _output_get (set `self.thirst` (`KismetMathLibrary.FClamp` (- (`self.thirst`) thirstAmount) 0.0 _maxthirst)))
  (`self.onThirstChanged` _output_get _maxthirst))