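; Player character component that tracks a Hunger value, draining it over time and restoring it when food is eaten.
; From BeginPlay, a self-calling Delay loop lowers Hunger by one every three seconds through UpdateHunger, while Eat adds to it.
; Both functions clamp between zero and MaxHunger and broadcast OnHungerChanged.
; UpdateHunger recomputes the subtraction for its broadcast, so listeners receive a value decremented twice.
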(event `self.ReceiveBeginPlay`
  (`self.decrementHunger`))

(event `decrementHunger`
  (`self.updateHunger` 1.0)
  (`KismetSystemLibrary.Delay` 3.0)
  (`self.decrementHunger`))

(fn `eat`
  (params (hungerAmount :type "Float (double-precision)"))
  (bind _maxhunger (`self.maxHunger`))
  (bind _output_get (set `self.hunger` (`KismetMathLibrary.FClamp` (+ hungerAmount (`self.hunger`)) 0.0 _maxhunger)))
  (`self.onHungerChanged` _output_get _maxhunger))

(fn `updateHunger`
  (params (foodAmount :type "Float (double-precision)"))
  (bind _maxhunger (`self.maxHunger`))
  (bind _returnvalue (`KismetMathLibrary.FClamp` (- (`self.hunger`) foodAmount) 0.0 _maxhunger))
  (set `self.hunger` _returnvalue)
  (`self.onHungerChanged` _returnvalue _maxhunger))