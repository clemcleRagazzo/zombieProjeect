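; Game mode that handles the game-over screen and restarting the player afterward.
; BeginPlay caches the player state, then fetches the controller and character through message calls.
; GameOver shows WBP_GameOver with UI-only input and a visible cursor.
; RestartAtCheckpoint teleports the character to a hardcoded location instead of a saved checkpoint, restores game input and walking, and removes the widget.
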(event `self.ReceiveBeginPlay`
  (bind _asbp_player_state (cast `/Game/PlayerCharacter/BP_PlayerState` (`GameplayStatics.GetPlayerState` 0)))
  (set `self.As BP Player State` _asbp_player_state)
  (bind _playercontroller (message `/Game/PlayerCharacter/Interfaces/BPI_PlayerCharacterLink.getPlayerController` (`GameplayStatics.GetPlayerController` 0)))
  (set `self.Player Controller` _playercontroller)
  (bind _playercharacter (message `/Game/PlayerCharacter/Interfaces/BPI_PlayerCharacterLink.getPlayerCharacter` (`GameplayStatics.GetPlayerCharacter` 0)))
  (set `self.Player Character` _playercharacter))

(fn `gameOver`
  (bind _player_controller (`self.Player Controller`))
  (bind _returnvalue (`|CreateWidget` "/Game/HUD/WBP_GameOver.WBP_GameOver_C"))
  (bind _output_get (set `self.gameOverUI` _returnvalue))
  (`UserWidget.AddToViewport` _returnvalue 0)
  (`UserWidget.AddToViewport` _output_get 0)
  (`WidgetBlueprintLibrary.SetInputMode_UIOnlyEx` _player_controller null)
  (set `PlayerController.bShowMouseCursor` true _player_controller))

(fn `getPlayerCharacter`
  (returns (PlayerCharacter :type "/Game/PlayerCharacter/BP_PlayerCharacter Object Reference"))
  (return null))

(fn `getPlayerController`
  (returns (playerController :type "/Game/PlayerCharacter/BP_PlayerController Object Reference"))
  (return null))

(fn `getPlayerGameMode`
  (returns (gameMode :type "/Game/PlayerCharacter/BP_PlayerGameMode Object Reference"))
  (return self))

(fn `getPlayerState`
  (returns (playerState :type "/Game/PlayerCharacter/BP_PlayerState Object Reference"))
  (return null))

(fn `restartAtCheckpoint`
  (bind _player_controller (`self.Player Controller`))
  (`self.resurrect`)
  (`WidgetBlueprintLibrary.SetInputMode_GameOnly` _player_controller)
  (set `PlayerController.bShowMouseCursor` false _player_controller)
  (`Widget.RemoveFromParent` (`self.gameOverUI`))
  (`CharacterMovementComponent.SetMovementMode` (`Character.CharacterMovement` (`self.Player Character`)) "MOVE_Walking" 0))

(fn `resurrect`
  (`self.K2_TeleportTo` :`self` (`self.Player Character`) :`DestLocation` (0.0 0.0 690.0)))

(fn `UserConstructionScript`)