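; Health component in the PlayerCharacter folder that handles damage, healing and death through OnHealthChanged and OnDeath dispatchers.
; TakeDammage and Heal do nothing once IsDead reports zero health.
; Damage clamps and stores CurrentHealth, broadcasting death at zero or a health change otherwise.
; Heal only broadcasts the unclamped sum without storing it, and Die broadcasts death without changing health.
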(fn `die`
  (returns (isDead :type Boolean))
  (`self.onDeath`)
  (return true))

(fn `heal`
  (params (healAmount :type "Float (double-precision)"))
  (bind _isdead (`self.isDead`))
  (if _isdead
    (return)
    (else
      (`self.onHealthChanged` (+ healAmount (`self.currentHealth`)) (`self.maxHealth`)))))

(fn `isDead`
  (returns (isDead :type Boolean))
  (return (<= (`self.currentHealth`) 0.0)))

(fn `takeDammage`
  (params (dammageAmount :type "Float (double-precision)"))
  (bind _maxhealth (`self.maxHealth`))
  (bind _isdead (`self.isDead`))
  (if _isdead
    (return)
    (else
      (bind _output_get (set `self.currentHealth` (`KismetMathLibrary.FClamp` (- (`self.currentHealth`) dammageAmount) 0.0 _maxhealth)))
      (if (== _output_get 0.0)
        (`self.onDeath`)
        (else
          (`self.onHealthChanged` _output_get _maxhealth))))))