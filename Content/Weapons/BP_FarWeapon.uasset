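; BP_FarWeapon is a ranged weapon that fires bullets, built on a parent that exposes first and second actions.
; The first action calls the parent version, then Shoot, which spawns a Bullet at the BulletSpawner component's world transform.
; The second action calls the parent version, then Aim, which so far only prints debug text.
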(fn `aim`
  (`KismetSystemLibrary.PrintText` "Viser"))

(fn `firstAction`
  (`parent.firstAction`)
  (`self.shoot`))

(fn `secondAction`
  (`parent.secondAction`)
  (`self.aim`))

(fn `shoot`
  (`KismetSystemLibrary.PrintText` "Tirer")
  (`|SpawnActorFromClass` (`self.bullet`) (`SceneComponent.K2_GetComponentToWorld` (`self.BulletSpawner`)) "Undefined" "MultiplyWithRoot" null null))

(fn `UserConstructionScript`)