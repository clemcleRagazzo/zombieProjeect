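; BP_HandWeapon is a weapon that registers itself as the player's nearby weapon and offers hit and block actions.
; A detection sphere sets NearedWeapon on BP_PlayerCharacter when overlap begins, then clears it half a second after overlap ends, whichever weapon it holds.
; FirstAction and SecondAction extend their parent versions with Hit and Block, which currently only print debug text.
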(event `self.SphereDetection_0.OnComponentBeginOverlap`
  (params (OverlappedComponent :type "PrimitiveComponent Object Reference") (OtherActor :type "Actor Object Reference") (OtherComp :type "PrimitiveComponent Object Reference") (OtherBodyIndex :type Integer) (bFromSweep :type Boolean) (SweepResult :type "HitResult Structure (by ref)"))
  ; Détection - entrée
  (bind _asbp_player_character (cast `/Game/PlayerCharacter/Blueprints/BP_PlayerCharacter` OtherActor))
  (set `/Game/PlayerCharacter/Blueprints/BP_PlayerCharacter.nearedWeapon` self _asbp_player_character)
  (`KismetSystemLibrary.PrintText` "arme définie"))

(event `self.SphereDetection_0.OnComponentEndOverlap`
  (params (OverlappedComponent :type "PrimitiveComponent Object Reference") (OtherActor :type "Actor Object Reference") (OtherComp :type "PrimitiveComponent Object Reference") (OtherBodyIndex :type Integer))
  ; Détection sortie
  (`KismetSystemLibrary.Delay` 0.5)
  (bind _asbp_player_character (cast `/Game/PlayerCharacter/Blueprints/BP_PlayerCharacter` OtherActor))
  (set `/Game/PlayerCharacter/Blueprints/BP_PlayerCharacter.nearedWeapon` null _asbp_player_character))

(fn `block`
  (`KismetSystemLibrary.PrintText` "Bloquer"))

(fn `firstAction`
  (`parent.firstAction`)
  (`self.hit`))

(fn `hit`
  (`KismetSystemLibrary.PrintText` "Taper"))

(fn `secondAction`
  (`parent.secondAction`)
  (`self.block`))

(fn `UserConstructionScript`)