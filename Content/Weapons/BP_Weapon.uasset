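; BP_Weapon is a weapon actor that the third-person character can detect nearby and that can be dropped into the world.
; Overlapping SphereDetection sets the character's NearedWeapon to this weapon, and leaving clears it after a short delay, without checking which weapon is stored.
; Drop re-enables collision on the weapon and sphere, turns on physics simulation and applies a zero impulse to the sphere, with debug prints.
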(event `self.SphereDetection.OnComponentBeginOverlap`
  (params (OverlappedComponent :type "PrimitiveComponent Object Reference") (OtherActor :type "Actor Object Reference") (OtherComp :type "PrimitiveComponent Object Reference") (OtherBodyIndex :type Integer) (bFromSweep :type Boolean) (SweepResult :type "HitResult Structure (by ref)"))
  ; Détection - entrée
  (bind _asbp_third_person_character (cast `/Game/ThirdPerson/Blueprints/BP_ThirdPersonCharacter` OtherActor))
  (set `/Game/ThirdPerson/Blueprints/BP_ThirdPersonCharacter.nearedWeapon` self _asbp_third_person_character)
  (`KismetSystemLibrary.PrintText` "arme définie"))

(event `self.SphereDetection.OnComponentEndOverlap`
  (params (OverlappedComponent :type "PrimitiveComponent Object Reference") (OtherActor :type "Actor Object Reference") (OtherComp :type "PrimitiveComponent Object Reference") (OtherBodyIndex :type Integer))
  ; Détection sortie
  (`KismetSystemLibrary.Delay` 0.5)
  (bind _asbp_third_person_character (cast `/Game/ThirdPerson/Blueprints/BP_ThirdPersonCharacter` OtherActor))
  (set `/Game/ThirdPerson/Blueprints/BP_ThirdPersonCharacter.nearedWeapon` null _asbp_third_person_character))

(fn `drop`
  (bind _weapon (`self.Weapon`))
  (bind _spheredetection (`self.SphereDetection`))
  (`PrimitiveComponent.SetCollisionEnabled` _weapon "QueryAndPhysics")
  (`PrimitiveComponent.SetSimulatePhysics` _weapon true)
  (`PrimitiveComponent.SetCollisionEnabled` _spheredetection "QueryAndPhysics")
  (`PrimitiveComponent.AddImpulse` _spheredetection (0.0 0.0 0.0) "hand_r" false)
  (`KismetSystemLibrary.PrintText` (`KismetTextLibrary.Conv_BoolToText` (`PrimitiveComponent.bGenerateOverlapEvents` _spheredetection))))

(fn `UserConstructionScript`)