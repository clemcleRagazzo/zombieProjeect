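; Lobby game mode that tracks joined players and provides kicking and server travel to a named level.
; Login and logout add or remove the player's lobby controller, then after a short delay tell the lobby game state to update its player list.
; Kicks go by list index to that controller.
; Getter functions resolve lobby classes; only the game mode getter returns a value, itself.
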(event `self.K2_PostLogin`
  (params (NewPlayer :type "PlayerController Object Reference"))
  (bind _lobbycontroller (message `/Game/HUD/Lobby/BPI_LobbyLinks.getLobbyController` NewPlayer))
  (`KismetArrayLibrary.Array_Add` (`self.joinedPlayersList`) _lobbycontroller)
  (`self.UpdatePlayersList` :!label _label))

(event `self.K2_OnLogout`
  (params (ExitingController :type "Controller Object Reference"))
  (bind _lobbycontroller (message `/Game/HUD/Lobby/BPI_LobbyLinks.getLobbyController` ExitingController))
  (`KismetArrayLibrary.Array_RemoveItem` (`self.joinedPlayersList`) _lobbycontroller)
  (goto _label))

(event `UpdatePlayersList`
  (`KismetSystemLibrary.Delay` 0.5)
  (bind _lobbygamestate (message `/Game/HUD/Lobby/BPI_LobbyLinks.getLobbyGameState` (`GameplayStatics.GetGameState`)))
  (`/Game/HUD/Lobby/GS_Lobby.UpdatePlayersList` _lobbygamestate))

(event `TravelTo`
  (params (LevelName :type String))
  (`AdvancedSessionsLibrary.ServerTravel` LevelName))

(fn `getLobbyController`
  (returns (lobbyController :type "/Game/HUD/Lobby/BP_LobbyController Object Reference"))
  (return null))

(fn `getLobbyGameMode`
  (returns (lobbyGameMode :type "/Game/HUD/Lobby/GM_Lobby Object Reference"))
  (return self))

(fn `getLobbyGameState`
  (returns (LobbyGameState :type "/Game/HUD/Lobby/GS_Lobby Object Reference"))
  (return null))

(fn `kickPlayer`
  (params (playerId :type Integer))
  (`/Game/HUD/Lobby/BP_LobbyController.kickPlayerOC` (`|GetArrayItem` (`self.joinedPlayersList`) playerId)))

(fn `UserConstructionScript`)