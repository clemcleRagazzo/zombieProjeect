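; Lobby player controller that shows the lobby UI and handles the player being kicked.
; On BeginPlay it creates and displays WBP_Lobby for the local controller only.
; The kick event opens the menu level, then destroys the session.
; Lobby getters expose the controller itself, while the game mode and game state getters return no value, and the view-target code is unconnected.
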(event `self.ReceiveBeginPlay`
  (if (`self.IsLocalController`)
    (bind _returnvalue (`|CreateWidget` "/Game/HUD/Lobby/WBP_Lobby.WBP_Lobby_C"))
    (`UserWidget.AddToViewport` _returnvalue 0)))

(event `kickPlayerOC`
  (`GameplayStatics.OpenLevelBySoftObjectPtr` "/Game/HUD/Menu/L_Menu.L_Menu")
  (`DestroySessionCallbackProxy.DestroySession` null))

(fn `getLobbyController`
  (returns (lobbyController :type "/Game/HUD/Lobby/BP_LobbyController Object Reference"))
  (return self))

(fn `getLobbyGameMode`
  (returns (lobbyGameMode :type "/Game/HUD/Lobby/GM_Lobby Object Reference"))
  (return null))

(fn `getLobbyGameState`
  (returns (LobbyGameState :type "/Game/HUD/Lobby/GS_Lobby Object Reference"))
  (return null))

(fn `UserConstructionScript`)