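; BP_Item is a pickup item that can be interacted with, attached to the interactor's mesh socket and dropped.
; Interact runs on authority, setting IsPickedUp and attaching at SocketName, while Drop clears the flag.
; The flag's RepNotify toggles physics and collision, detaching on release.
; OnFocused shows the interact widget until a retriggerable delay lapses; first and second actions are empty stubs.
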(event `self.ReceiveBeginPlay`)

(event `/Game/PlayerCharacter/Interfaces/BPI_Interact.interact`
  (params (interactor :type "/Game/PlayerCharacter/BP_PlayerCharacter Object Reference"))
  (`/Engine/EditorBlueprintResources/ActorMacros.Switch Has Authority`
    (:`Authority`
      (set `self.bIsPickedUp ` true)
      (bind _returnvalue (`self.K2_AttachToComponent` (`Character.Mesh` interactor) (`self.socketName`) "SnapToTarget" "SnapToTarget" "SnapToTarget"))
      (if _returnvalue
        _))))

(event `Drop`
  (set `self.bIsPickedUp ` false))

(event `/Game/PlayerCharacter/Interfaces/BPI_Interact.onFocused`
  (`SceneComponent.SetVisibility` (`self.WBP_Interact`) true false)
  (`KismetSystemLibrary.RetriggerableDelay` 0.2)
  (`SceneComponent.SetVisibility` (`self.WBP_Interact`) false false))

(fn `firstAction`)

(fn `getItem`
  (returns (item :type "/Game/Items/BP_Item Object Reference"))
  (return self))

(fn `OnRep_bIsPickedUp `
  (bind _item (`self.Item`))
  (bind _item_2 (`self.Item`))
  (if (`self.bIsPickedUp `)
    (`PrimitiveComponent.SetSimulatePhysics` _item_2 false)
    (`PrimitiveComponent.SetCollisionEnabled` _item_2 "NoCollision")
    (else
      (`SceneComponent.K2_DetachFromComponent` _item "KeepWorld" "KeepWorld" "KeepWorld" true)
      (`PrimitiveComponent.SetSimulatePhysics` _item true)
      (`PrimitiveComponent.SetCollisionEnabled` _item "QueryAndPhysics")
      (`PrimitiveComponent.AddImpulse` _item (0.0 0.0 0.0) (`self.socketName`) false))))

(fn `secondAction`)

(fn `UserConstructionScript`)