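; BP_Consummable is an inventory system item, typically a consumable, that heals the player character when interacted with.
; Interact checks the item type in its Datas struct and, for Consummable, plays the heal sound and applies the heal amount to the player's health component.
; The construction script sets the static mesh from the same data and applies a uniform MeshScale.
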(event `self.interact`
  (params (interactor :type "/Game/PlayerCharacter/BP_PlayerCharacter Object Reference"))
  (bind _datas (`self.datas`))
  (bind (_canheal _healamount _healfx _healsound) (break `/Game/Blueprints/InventorySystem/SP_ConsummableData` (`/Game/Blueprints/InventorySystem/PDA_InventorySystem.consummableData` _datas)))
  (switch `/Game/Blueprints/InventorySystem/E_ItemType` (`/Game/Blueprints/InventorySystem/PDA_InventorySystem.type` _datas)
    (:`NewEnumerator1`
      (`GameplayStatics.PlaySound2D` _healsound 1.0 1.0 0.0 null null)
      (`/Game/PlayerCharacter/ActorsComponent/AC_HealthComponent.heal` (`/Game/PlayerCharacter/BP_PlayerCharacter.AC_HealthComponent` (`self.As BP Player Character`)) _healamount))))

(fn `UserConstructionScript`
  (`StaticMeshComponent.SetStaticMesh` (`self.StaticMesh`) (`/Game/Blueprints/InventorySystem/PDA_InventorySystem.mesh` (`self.datas`)))
  (`SceneComponent.SetRelativeScale3D` (`self.StaticMesh`) (`KismetMathLibrary.Conv_DoubleToVector` (`self.meshScale`))))